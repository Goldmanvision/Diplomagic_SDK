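; Exit-stairs room piece for the procedurally generated dungeon, which sends the player out of the level.
; When a BP_ProtoPlayer overlaps the LevelExit component, it plays a sound, waits briefly, then opens the DM_Plane_Test level.
; Unconnected leftover logic would destroy all room and wall-gap actors or have the owning Dungeon_Generator spawn more rooms, but it never runs.
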(event `self.levelExit.OnComponentBeginOverlap`
  (params (OverlappedComponent :type "PrimitiveComponent Object Reference") (OtherActor :type "Actor Object Reference") (OtherComp :type "PrimitiveComponent Object Reference") (OtherBodyIndex :type Integer) (bFromSweep :type Boolean) (SweepResult :type "HitResult Structure (by ref)"))
  (bind _asbp_proto_player (cast `/Game/Dynamic/Blueprints/BP_ProtoPlayer` OtherActor))
  (`GameplayStatics.PlaySound2D` "/Engine/VREditor/Sounds/UI/Enter_Simulate.Enter_Simulate" 1.0 1.0 0.0 null _asbp_proto_player)
  (`KismetSystemLibrary.Delay` 1.0)
  (`GameplayStatics.OpenLevelBySoftObjectPtr` "/Game/Dynamic/Maps/DM_Plane_Test.DM_Plane_Test"))

(fn `UserConstructionScript`
  (`parent.UserConstructionScript`))