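; BP_lighting_strike is a Paper2D flipbook actor, named as a lightning strike effect, that billboards its sprite toward the player camera.
; Every tick it sets the flipbook's world yaw from a look-at rotation to the camera, offset by 90 degrees, keeping pitch and roll at zero.
; A directional sprite angle calculation sits behind a constant-true branch and never runs, and a left/right side test is left unused.
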(event `self.ReceiveTick`
  (params (DeltaSeconds :type "Float (single-precision)"))
  (bind (_returnvalue_x _returnvalue_y) (`KismetMathLibrary.BreakVector` (`self.GetActorForwardVector`)))
  (bind (_returnvalue_x_2 _returnvalue_y_2) (`KismetMathLibrary.BreakVector` (`self.K2_GetActorLocation`)))
  (bind (_returnvalue_x_3 _returnvalue_y_3) (`KismetMathLibrary.BreakVector` (`self.K2_GetActorLocation` (`GameplayStatics.GetPlayerCameraManager` 0))))
  (bind (_returnvalue_roll _returnvalue_pitch _returnvalue_yaw) (`KismetMathLibrary.BreakRotator` (`KismetMathLibrary.FindLookAtRotation` (`SceneComponent.K2_GetComponentLocation` (`self.PaperFlipbook`)) (`PlayerCameraManager.GetCameraLocation` (`GameplayStatics.GetPlayerCameraManager` 0)))))
  ;[0 1 0 1 32] Sprite Face Camera
  (`SceneComponent.K2_SetWorldRotation` (`self.PaperFlipbook`) (`KismetMathLibrary.MakeRotator` 0.0 0.0 (- _returnvalue_yaw 90.0)) false false)
  (if (not true)
    (set `self.SpriteAngle` (`KismetMathLibrary.DegAcos` (`KismetMathLibrary.Dot_VectorVector` (`KismetMathLibrary.MakeVector` _returnvalue_x _returnvalue_y) (`KismetMathLibrary.Normal` (- (`KismetMathLibrary.MakeVector` _returnvalue_x_3 _returnvalue_y_3) (`KismetMathLibrary.MakeVector` _returnvalue_x_2 _returnvalue_y_2))))))))

(fn `UserConstructionScript`)