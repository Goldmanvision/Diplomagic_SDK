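; Paper2D NPC character, apparently derived from a prototype player, that shows directional flipbook sprites in a 3D world.
; Macros compute the angle between the actor's facing and the player pawn, pick front, side or back flipbooks from it, and yaw-billboard the sprite toward the camera.
; Other helpers cover compass movement input, dash destination and trace, velocity checks and an on-screen controls help printout.
; No event graph here calls these helpers.
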(fn `DashTraceLength`
  (returns (Start :type "Vector Structure") (End :type "Vector Structure"))
  (bind _returnvalue (`self.K2_GetActorLocation`))
  (return _returnvalue (+ _returnvalue (* (`self.Directionality`) (`self.TraceDistance`)))))

(fn `Determine Dash Destination`
  (params (DashDistance :type "Float (double-precision)") (Directionality :type "Vector2D Structure"))
  (returns (`Dash Destination` :type "Vector Structure"))
  (return (+ (* (`self.Directionality`) (`self.DashDistance`)) (`self.K2_GetActorLocation`))))

(fn `hasNoVelocity`
  (returns (OutputPin :type Boolean))
  (return (and (`KismetMathLibrary.NearlyEqual_FloatFloat` (.x (`self.GetVelocity`))) (`KismetMathLibrary.NearlyEqual_FloatFloat` (.y (`self.GetVelocity`))))))

(fn `isLowVelocity`
  (returns (ReturnValue :type Boolean))
  (bind _returnvalue (> (`KismetMathLibrary.Abs` (.y (`self.GetVelocity`))) 200.0))
  (bind _returnvalue_2 (> (`KismetMathLibrary.Abs` (.x (`self.GetVelocity`))) 200.0))
  (return (xor (xor _returnvalue_2 _returnvalue) (and _returnvalue_2 _returnvalue))))

(fn `PrintVelocityAndDirectionality`
  (bind (_directionality_x _directionality_y) (`KismetMathLibrary.BreakVector2D` (`self.Directionality`)))
  (`KismetSystemLibrary.PrintString` (`KismetStringLibrary.Concat_StrStr` "VECTOR X: " (`KismetStringLibrary.Conv_DoubleToString` (.x (`self.GetVelocity`))) ", VECTOR Y: " (`KismetStringLibrary.Conv_DoubleToString` (.y (`self.GetVelocity`))) ", DIRECTIONALITY X:" (`KismetStringLibrary.Conv_DoubleToString` _directionality_x) ", DIRECTIONALITY Y:" (`KismetStringLibrary.Conv_DoubleToString` _directionality_y))))

(fn `ShowHelp`
  (`KismetSystemLibrary.PrintString` "QUIT GAME -- ESC or ALT-F4" true false (make `LinearColor` (`KismetMathLibrary.FClamp` (`KismetMathLibrary.RandomFloat`) (`self.ColorClampMin`) (`self.ColorClampMax`)) (`KismetMathLibrary.FClamp` (`KismetMathLibrary.RandomFloat`) (`self.ColorClampMin`) (`self.ColorClampMax`)) (`KismetMathLibrary.FClamp` (`KismetMathLibrary.RandomFloat`) (`self.ColorClampMin`) (`self.ColorClampMax`))) 17.5)
  (`KismetSystemLibrary.PrintString` "--------------------------- \n \nSHOW CONTROLS -- H \nRESET LEVEL -- ENTER \n \n--------------------------- \n" true false (make `LinearColor` (`KismetMathLibrary.FClamp` (`KismetMathLibrary.RandomFloat`) (`self.ColorClampMin`) (`self.ColorClampMax`)) (`KismetMathLibrary.FClamp` (`KismetMathLibrary.RandomFloat`) (`self.ColorClampMin`) (`self.ColorClampMax`)) (`KismetMathLibrary.FClamp` (`KismetMathLibrary.RandomFloat`) (`self.ColorClampMin`) (`self.ColorClampMax`))) 18.0)
  (`KismetSystemLibrary.PrintString` "MOVE -- ARROW KEYS \nFLIP CAMERA / FLIP ROLL DIRECTION -- Q or E \nJUMP / DOUBLE JUMP -- SPACEBAR \nROLL -- W \n" true false (make `LinearColor` (`KismetMathLibrary.FClamp` (`KismetMathLibrary.RandomFloat`) (`self.ColorClampMin`) (`self.ColorClampMax`)) (`KismetMathLibrary.FClamp` (`KismetMathLibrary.RandomFloat`) (`self.ColorClampMin`) (`self.ColorClampMax`)) (`KismetMathLibrary.FClamp` (`KismetMathLibrary.RandomFloat`) (`self.ColorClampMin`) (`self.ColorClampMax`))) 18.5)
  (`KismetSystemLibrary.PrintString` (`KismetStringLibrary.Concat_StrStr` " \n--------------------------- \nKEYBOARD \n" "--------------------------- \n") true false (make `LinearColor` (`KismetMathLibrary.FClamp` (`KismetMathLibrary.RandomFloat`) (`self.ColorClampMin`) (`self.ColorClampMax`)) (`KismetMathLibrary.FClamp` (`KismetMathLibrary.RandomFloat`) (`self.ColorClampMin`) (`self.ColorClampMax`)) (`KismetMathLibrary.FClamp` (`KismetMathLibrary.RandomFloat`) (`self.ColorClampMin`) (`self.ColorClampMax`))) 19.0)
  (`KismetSystemLibrary.PrintString` "MOVE  --  LEFT THUMBSTICK \nROTATE CAMERA -- LEFT THUMBSTICK CLICK or RIGHT SHOULDER \nJUMP / DOUBLE JUMP -- BOTTOM FACE BUTTON \nROLL -- RIGHT FACE BUTTON \nSHOW HELP -- START BUTTON \nRESET LEVEL -- BACK BUTTON" true false (make `LinearColor` (`KismetMathLibrary.FClamp` (`KismetMathLibrary.RandomFloat`) (`self.ColorClampMin`) (`self.ColorClampMax`)) (`KismetMathLibrary.FClamp` (`KismetMathLibrary.RandomFloat`) (`self.ColorClampMin`) (`self.ColorClampMax`)) (`KismetMathLibrary.FClamp` (`KismetMathLibrary.RandomFloat`) (`self.ColorClampMin`) (`self.ColorClampMax`))) 19.5)
  (`KismetSystemLibrary.PrintString` (`KismetStringLibrary.Concat_StrStr` "--------------------------- \nGAMEPAD \n" "--------------------------- \n") true false (make `LinearColor` (`KismetMathLibrary.FClamp` (`KismetMathLibrary.RandomFloat`) 0.2 0.8) (`KismetMathLibrary.FClamp` (`KismetMathLibrary.RandomFloat`) 0.2 0.8) (`KismetMathLibrary.FClamp` (`KismetMathLibrary.RandomFloat`) 0.2 0.8)) 20.0))

(fn `UserConstructionScript`)