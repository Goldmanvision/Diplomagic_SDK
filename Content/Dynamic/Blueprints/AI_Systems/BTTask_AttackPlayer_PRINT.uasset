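; Behavior Tree task for an AI attack on the player, with gunshot, hurt and bullet-impact feedback.
; A DoOnce gates the attack, which subtracts Health through the player's BPC_Attributes and runs a debug-drawn line trace to place the impact sound.
; The task finishes only when Health is already below zero.
; Ghoul-bite prints and the ResetAttack call are disconnected.
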(event `ResetAttack`
  (bind _returnvalue (`GameplayStatics.GetPlayerCharacter` 0))
  (bind _returnvalue_2 (`Actor.GetComponentByClass` _returnvalue "/Game/Dynamic/Blueprints/RPG_Systems/Attributes/BPC_Attributes.BPC_Attributes_C"))
  (bind _health_basevalue (break `/Game/Dynamic/Blueprints/RPG_Systems/Attributes/S_Attribute` (`/Game/Dynamic/Blueprints/RPG_Systems/Attributes/BPC_Attributes.Health` _returnvalue_2)))
  (goto _label :!via `Reset`))

(event `self.ReceiveExecuteAI`
  (params (OwnerController :type "AIController Object Reference") (ControlledPawn :type "Pawn Object Reference"))
  (bind _returnvalue (`GameplayStatics.GetPlayerCharacter` 0))
  (bind _returnvalue_2 (`Actor.K2_GetActorLocation` OwnerController))
  (bind _returnvalue_3 (`Actor.GetComponentByClass` _returnvalue "/Game/Dynamic/Blueprints/RPG_Systems/Attributes/BPC_Attributes.BPC_Attributes_C"))
  (bind _health_basevalue (break `/Game/Dynamic/Blueprints/RPG_Systems/Attributes/S_Attribute` (`/Game/Dynamic/Blueprints/RPG_Systems/Attributes/BPC_Attributes.Health` _returnvalue_3)))
  (`/Engine/EditorBlueprintResources/StandardMacros.DoOnce` false :!label _label
    (:`Completed`
      (`GameplayStatics.PlaySoundAtLocation` "/Game/Dynamic/Sound/Audio/080978_fully-automatic-pistol-uzi-39778.080978_fully-automatic-pistol-uzi-39778" _returnvalue_2 (struct) 1.0 (`KismetMathLibrary.RandomFloatInRange` 0.8 1.2) 0.0 null null OwnerController null)
      (if (>= _health_basevalue 0.0)
        (`/Game/Dynamic/Blueprints/RPG_Systems/Attributes/BPC_Attributes.ChangeAttribute` _returnvalue_3 (struct :`TagName` "Attribute.Health") -10.0 "NewEnumerator1" (make `/Game/Dynamic/Blueprints/S_Origin` _returnvalue OwnerController))
        (`GameplayStatics.PlaySound2D` "/Game/Dynamic/Sound/Audio/breaking-small-bone-finger-88085.breaking-small-bone-finger-88085" 0.85 (`KismetMathLibrary.RandomFloatInRange` 0.8 1.2) 0.0 null null)
        (`GameplayStatics.PlaySound2D` "/Game/Dynamic/Sound/Audio/hurt_sounds_cue.hurt_sounds_cue" 1.2 1.0 0.0 null null)
        (`GameplayStatics.SpawnForceFeedbackAtLocation` "/Game/Dynamic/Input/Controller_Systems/FireWeapon.FireWeapon" (`.ImpactPoint` (`GameplayStatics.BreakHitResult` (stale _outhit))) (struct) false 1.0 0.0 null)
        (bind _outhit (`KismetSystemLibrary.LineTraceSingle` :`Start` _returnvalue_2 :`End` (`Actor.K2_GetActorLocation` _returnvalue) :`TraceChannel` "TraceTypeQuery1" :`DrawDebugType` "ForDuration" :`TraceColor` (struct :`R` 0.911281 :`G` 1.0 :`A` 1.0) :`TraceHitColor` (struct :`R` 1.0 :`A` 1.0) :`DrawTime` 1.0))
        (`GameplayStatics.PlaySoundAtLocation` "/Game/Dynamic/Sound/Audio/080998_bullet-hit-39870.080998_bullet-hit-39870" (`.Location` (`GameplayStatics.BreakHitResult` _outhit)) (struct) 1.0 (`KismetMathLibrary.RandomFloatInRange` 0.8 1.2) 0.0 null null OwnerController null)
        (else
          (`self.FinishExecute` true))))))