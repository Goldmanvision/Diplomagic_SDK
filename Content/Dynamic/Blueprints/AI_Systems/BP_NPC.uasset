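; BP_NPC is an NPC character drawn as an eight-directional 2D flipbook sprite in a 3D world.
; Each Tick it yaws the sprite toward the player camera, then, unless dead or paused, checks velocity to choose running or idle.
; Dot products of the actor's forward and right vectors with the camera direction give angle and side, which SetSpriteFacing and SetFlipbook turn into the matching flipbook.
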(event `self.ReceiveTick`
  (params (DeltaSeconds :type "Float (single-precision)"))
  (bind (_returnvalue_x _returnvalue_y) (`KismetMathLibrary.BreakVector` (`self.GetActorRightVector`)))
  (bind (_returnvalue_x_2 _returnvalue_y_2) (`KismetMathLibrary.BreakVector` (`self.GetActorForwardVector`)))
  (bind (_returnvalue_x_3 _returnvalue_y_3) (`KismetMathLibrary.BreakVector` (`self.K2_GetActorLocation`)))
  (bind _spriteangle (`self.SpriteAngle`))
  (bind (_returnvalue_x_4 _returnvalue_y_4) (`KismetMathLibrary.BreakVector` (`self.K2_GetActorLocation` (`GameplayStatics.GetPlayerCameraManager` 0))))
  (bind (_returnvalue_roll _returnvalue_pitch _returnvalue_yaw) (`KismetMathLibrary.BreakRotator` (`KismetMathLibrary.FindLookAtRotation` (`SceneComponent.K2_GetComponentLocation` (`self.Sprite`)) (`PlayerCameraManager.GetCameraLocation` (`GameplayStatics.GetPlayerCameraManager` 0)))))
  (bind _returnvalue (`KismetMathLibrary.Normal` (- (`KismetMathLibrary.MakeVector` _returnvalue_x_4 _returnvalue_y_4) (`KismetMathLibrary.MakeVector` _returnvalue_x_3 _returnvalue_y_3))))
  ;[0 1 0 1 32] Sprite Face Camera
  (`SceneComponent.K2_SetWorldRotation` (`self.Sprite`) (`KismetMathLibrary.MakeRotator` 0.0 0.0 (- _returnvalue_yaw 90.0)) false false)
  (if (not (or (`self.Is Dead`) (`self.Pause Angle Calculation`)))
    (`self.CheckIfRunning`
      (:`Out`
        ;[0 1 0 1 32] Set Sprite Flipbook
        (set `self.SpriteAngle` (`KismetMathLibrary.DegAcos` (`KismetMathLibrary.Dot_VectorVector` (`KismetMathLibrary.MakeVector` _returnvalue_x_2 _returnvalue_y_2) _returnvalue)))
        (if (< (`KismetMathLibrary.Dot_VectorVector` _returnvalue (`KismetMathLibrary.MakeVector` _returnvalue_x _returnvalue_y)) 0.0)
          (set `self.Sprite_Left_Side_Visible` true)
          (else
            (set `self.Sprite_Left_Side_Visible` false)))
        (if (< _spriteangle 22.5)
          (`self.SetSpriteFacing` "NewEnumerator0")
          (elif (< _spriteangle 67.5)
            (`self.SetSpriteFacing` "NewEnumerator1")
            (elif (< _spriteangle 112.5)
              (`self.SetSpriteFacing` "NewEnumerator2")
              (elif (< _spriteangle 157.5)
                (`self.SetSpriteFacing` "NewEnumerator3")
                (else
                  (`self.SetSpriteFacing` "NewEnumerator4"))))))))))

(fn `SetFlipbook`
  (params (Running :type "PaperFlipbook Object Reference") (Idle :type "PaperFlipbook Object Reference"))
  (bind _sprite (`self.Sprite`))
  (if (`self.Is Running`)
    (`PaperFlipbookComponent.SetFlipbook` _sprite Running)
    (else
      (`PaperFlipbookComponent.SetFlipbook` _sprite Idle))))

(fn `SetSpriteFacing`
  (params (Facing :type "/Game/Dynamic/Blueprints/ENUM_NPC_Facing Enum" :default "NewEnumerator0"))
  (switch `/Game/Dynamic/Blueprints/ENUM_NPC_Facing` Facing
    (:`NewEnumerator0`
      (`self.SetFlipbook` (`self.Run_Front`) (`self.Idle_Front`)))
    (:`NewEnumerator1`
      (if (`self.Sprite_Left_Side_Visible`)
        (`self.SetFlipbook` (`self.Run_Front-Left`) (`self.Idle_Front-Left`))
        (else
          (`self.SetFlipbook` (`self.Run_Front-Right`) (`self.Idle_Front-Right`)))))
    (:`NewEnumerator2`
      (if (`self.Sprite_Left_Side_Visible`)
        (`self.SetFlipbook` (`self.Run_Left`) (`self.Idle_Left`))
        (else
          (`self.SetFlipbook` (`self.Run_Right`) (`self.Idle_Right`)))))
    (:`NewEnumerator3`
      (if (`self.Sprite_Left_Side_Visible`)
        (`self.SetFlipbook` (`self.Run_Back-Left`) (`self.Idle_Back-Left`))
        (else
          (`self.SetFlipbook` (`self.Run_Back-Right`) (`self.Idle_Back-Right`)))))
    (:`NewEnumerator4`
      (`self.SetFlipbook` (`self.Run_Back`) (`self.Idle_Back`)))))

(fn `UserConstructionScript`)