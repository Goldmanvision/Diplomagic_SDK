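; Master gem pickup that awards XP to BP_ProtoPlayer's BPC_XP component on overlap, plays a sound and destroys itself.
; BeginPlay randomizes flipbook color, matching light, position offset and scale through a DoOnce, spread across ticks.
; Tick billboards the sprite toward the camera on yaw only and stores its viewing angle in SpriteAngle.
; Non-player overlaps apply a small upward impulse to the collision box.
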(event `ResetRandomizer`
  (bind (_outitem _outindex) (`KismetArrayLibrary.Array_Random` (`|MakeArray` (`self.gem_red`) (`self.gem_blue`) (`self.gem_green`) (`self.gem_yellow`))))
  (goto _label :!via `Reset`))

(event `self.ReceiveBeginPlay`
  (bind (_outitem _outindex) (`KismetArrayLibrary.Array_Random` (`|MakeArray` (`self.gem_red`) (`self.gem_blue`) (`self.gem_green`) (`self.gem_yellow`))))
  (`/Engine/EditorBlueprintResources/StandardMacros.DoOnce` false :!label _label
    (:`Completed`
      (set `self.ArrayElement` _outindex)
      (`KismetSystemLibrary.DelayUntilNextTick`)
      (`PaperFlipbookComponent.SetFlipbook` (`self.gem_FB`) _outitem)
      (`KismetSystemLibrary.DelayUntilNextTick`)
      (`LightComponent.SetLightColor` (`self.gem_PL`) (`|GetArrayItem` (`|MakeArray` (`self.gem_red_light`) (`self.gem_blue_light`) (`self.gem_green_light`) (`self.gem_yellow_light`)) (`self.ArrayElement`)) true)
      (`KismetSystemLibrary.DelayUntilNextTick`)
      (`self.K2_SetActorTransform` (`KismetMathLibrary.MakeTransform` (+ (`KismetMathLibrary.RandomFloatInRange` 3.0 10.0) (`self.K2_GetActorLocation`)) (`self.K2_GetActorRotation`) (+ (`KismetMathLibrary.RandomFloatInRange` 3.0 6.0) (`self.GetActorScale3D`))))
      (`self.ResetRandomizer`))))

(event `self.ReceiveActorBeginOverlap`
  (params (OtherActor :type "Actor Object Reference"))
  (bind _returnvalue (`GameplayStatics.GetObjectClass` OtherActor))
  (if (and (== _returnvalue "/Game/Dynamic/Blueprints/BP_ProtoPlayer.BP_ProtoPlayer_C") (!= _returnvalue "/Script/Landscape.Landscape"))
    (`self.XP_ConsumablePickedUp` OtherActor)
    (else
      (`PrimitiveComponent.AddImpulse` (`self.gem_collisionBox`) (0.0 0.0 1.0) "None" false)
      (`KismetSystemLibrary.PrintString` "not a player"))))

(event `self.ReceiveTick`
  (params (DeltaSeconds :type "Float (single-precision)"))
  (bind (_returnvalue_x _returnvalue_y) (`KismetMathLibrary.BreakVector` (`self.GetActorForwardVector`)))
  (bind (_returnvalue_x_2 _returnvalue_y_2) (`KismetMathLibrary.BreakVector` (`self.K2_GetActorLocation`)))
  (bind (_returnvalue_x_3 _returnvalue_y_3) (`KismetMathLibrary.BreakVector` (`self.K2_GetActorLocation` (`GameplayStatics.GetPlayerCameraManager` 0))))
  (bind (_returnvalue_roll _returnvalue_pitch _returnvalue_yaw) (`KismetMathLibrary.BreakRotator` (`KismetMathLibrary.FindLookAtRotation` (`SceneComponent.K2_GetComponentLocation` (`self.gem_FB`)) (`PlayerCameraManager.GetCameraLocation` (`GameplayStatics.GetPlayerCameraManager` 0)))))
  ;[0 1 0 1 32] Sprite Face Camera
  (`SceneComponent.K2_SetWorldRotation` (`self.gem_FB`) (`KismetMathLibrary.MakeRotator` 0.0 0.0 (- _returnvalue_yaw 90.0)) false false)
  (set `self.SpriteAngle` (`KismetMathLibrary.DegAcos` (`KismetMathLibrary.Dot_VectorVector` (`KismetMathLibrary.MakeVector` _returnvalue_x _returnvalue_y) (`KismetMathLibrary.Normal` (- (`KismetMathLibrary.MakeVector` _returnvalue_x_3 _returnvalue_y_3) (`KismetMathLibrary.MakeVector` _returnvalue_x_2 _returnvalue_y_2)))))))

(fn `UserConstructionScript`)