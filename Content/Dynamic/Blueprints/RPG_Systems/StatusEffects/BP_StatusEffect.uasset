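; Base status effect for the RPG systems that applies gameplay tags to its owner for a set duration, with an empty periodic event.
; Application checks the owner's BPC_GameplayTags against requirement and prevention tags, removing the effect on failure.
; On success it adds its tags and starts a looping periodic timer plus a duration timer.
; When duration ends, it removes those tags, clears timers and removes itself through BPC_StatusEffects.
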(event `AttemptApplication`
  (bind _applystatuseffect (`self.CheckTagStartConditions`))
  (if _applystatuseffect
    (`self.StartStatusEffect`)
    (else
      (`self.AttemptStatusEffectRemoval`))))

(event `StartStatusEffect`
  (bind (_duration _periodictime) (break `/Game/Dynamic/Blueprints/RPG_Systems/StatusEffects/S_StatusEffect` (`self.StatusEffectInfo`)))
  (`self.AddTags`)
  (bind _returnvalue (`KismetSystemLibrary.K2_SetTimerDelegate` (delegate `PeriodicEvent`) _periodictime true))
  (set `self.PeriodicTimerHandle` _returnvalue)
  (bind _returnvalue_2 (`KismetSystemLibrary.K2_SetTimerDelegate` (delegate `EndStatusEffect`) _duration false false 0.001))
  (set `self.DurationTimerHandle` _returnvalue_2))

(event `PeriodicEvent`)

(event `EndStatusEffect`
  (`self.RemoveTags`)
  (`self.ClearTimers`)
  (`self.AttemptStatusEffectRemoval`))

(fn `AddTags`
  (bind _returnvalue (`self.GetOwner`))
  (for _array_element (`self.AddingTags`)
    (`/Game/Dynamic/Blueprints/GameplayTags/BPC_GameplayTags.AddTag` (`self.GetComponentByClass` _returnvalue "/Game/Dynamic/Blueprints/GameplayTags/BPC_GameplayTags.BPC_GameplayTags_C") _array_element (make `/Game/Dynamic/Blueprints/S_Origin` _returnvalue (`self.GetInstigatorController` _returnvalue))))
  (return))

(fn `CheckTagStartConditions`
  (returns (ApplyStatusEffect :type Boolean))
  (bind _tagcontainer (`/Game/Dynamic/Blueprints/GameplayTags/BPC_GameplayTags.GetActiveTagContainer` (`self.GetComponentByClass` (`self.GetOwner`) "/Game/Dynamic/Blueprints/GameplayTags/BPC_GameplayTags.BPC_GameplayTags_C")))
  (return (and (not (`BlueprintGameplayTagLibrary.HasAnyTags` _tagcontainer (`self.PreventionTags`))) (`BlueprintGameplayTagLibrary.HasAllTags` _tagcontainer (`self.RequirementTags`)))))

(fn `ClearTimers`
  (`KismetSystemLibrary.K2_ClearAndInvalidateTimerHandle` (`self.PeriodicTimerHandle`))
  (`KismetSystemLibrary.K2_ClearAndInvalidateTimerHandle` (`self.DurationTimerHandle`)))

(fn `RemoveTags`
  (bind _returnvalue (`self.GetOwner`))
  (for _array_element (`self.AddingTags`)
    (`/Game/Dynamic/Blueprints/GameplayTags/BPC_GameplayTags.RemoveTag` (`self.GetComponentByClass` _returnvalue "/Game/Dynamic/Blueprints/GameplayTags/BPC_GameplayTags.BPC_GameplayTags_C") _array_element (make `/Game/Dynamic/Blueprints/S_Origin` _returnvalue (`self.GetInstigatorController` _returnvalue))))
  (return))

(fn `UserConstructionScript`)