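; Actor component for the RPG attribute system that stores attributes and handles lookup, changes and listeners by tag, currently supporting only Health.
; The DetermineAttribute macro routes each tag to its attribute struct.
; ChangeAttribute adds a value to the chosen field (base, delta, multiplier or max) without clamping.
; It then broadcasts a per-attribute dispatcher with the attribute, change and origin, which AddAttributeListener binds to.
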(event `self.ReceiveBeginPlay`)

(event `Signature` :!signature `self.AttributeHealthChanged`
  (params (AttributeContext :type "/Game/Dynamic/Blueprints/RPG_Systems/Attributes/S_AttributeContext Structure")))

(fn `AddAttributeListener`
  (params (AttributeTag :type "GameplayTag Structure") (Event :type "Delegate (by ref)"))
  (`self.DetermineAttribute` AttributeTag
    (:`Health`
      (add `self.AttributeHealthChanged` Event))))

(fn `ChangeAttribute`
  (params (AttributeTag :type "GameplayTag Structure") (ValueChange :type "Float (double-precision)") (AttributeTypeToChange :type "/Game/Dynamic/Blueprints/RPG_Systems/Attributes/E_Attribute Enum" :default "NewEnumerator0") (Origin :type "/Game/Dynamic/Blueprints/S_Origin Structure"))
  (`self.DetermineAttribute` AttributeTag
    (:`Health`
      (`self.ChangeAttributeValue` (`self.Health`) (`local.ValueChange`) (`local.AttributeTypeToChange`))
      (bind _context (`self.CreateAttributeContext` (`self.Health`) (`local.ValueChange`) (`local.Origin`)))
      (`self.AttributeHealthChanged` _context)
      (return))
    (:`NoAttribute`)))

(fn `ChangeAttributeValue`
  (params (AttributeToChange :type "/Game/Dynamic/Blueprints/RPG_Systems/Attributes/S_Attribute Structure (by ref)") (ValueChange :type "Float (double-precision)") (AttributeTypeToChange :type "/Game/Dynamic/Blueprints/RPG_Systems/Attributes/E_Attribute Enum" :default "NewEnumerator0"))
  (bind (_basevalue _delta _multiplier _max) (break `/Game/Dynamic/Blueprints/RPG_Systems/Attributes/S_Attribute` AttributeToChange))
  (bind _valuechange (`local.ValueChange`))
  (switch `/Game/Dynamic/Blueprints/RPG_Systems/Attributes/E_Attribute` AttributeTypeToChange
    (:`NewEnumerator0`
      _)
    (:`NewEnumerator1`
      (setmembers `/Game/Dynamic/Blueprints/RPG_Systems/Attributes/S_Attribute` :`StructRef` AttributeToChange :`BaseValue` (+ _valuechange _basevalue)))
    (:`NewEnumerator2`
      (setmembers `/Game/Dynamic/Blueprints/RPG_Systems/Attributes/S_Attribute` :`StructRef` AttributeToChange :`Delta` (+ _delta _valuechange)))
    (:`NewEnumerator3`
      (setmembers `/Game/Dynamic/Blueprints/RPG_Systems/Attributes/S_Attribute` :`StructRef` AttributeToChange :`Multiplier` (+ _multiplier _valuechange)))
    (:`NewEnumerator4`
      (setmembers `/Game/Dynamic/Blueprints/RPG_Systems/Attributes/S_Attribute` :`StructRef` AttributeToChange :`Max` (+ _max _valuechange))))
  (return))

(fn `CreateAttributeContext`
  (params (AttributeChanged :type "/Game/Dynamic/Blueprints/RPG_Systems/Attributes/S_Attribute Structure") (ValueChange :type "Float (double-precision)") (Origin :type "/Game/Dynamic/Blueprints/S_Origin Structure"))
  (returns (Context :type "/Game/Dynamic/Blueprints/RPG_Systems/Attributes/S_AttributeContext Structure"))
  (return (make `/Game/Dynamic/Blueprints/RPG_Systems/Attributes/S_AttributeContext` AttributeChanged ValueChange Origin)))

(fn `GetAttributeFromTag`
  (params (TagSearchedFor :type "GameplayTag Structure"))
  (returns (AttributeFound :type "/Game/Dynamic/Blueprints/RPG_Systems/Attributes/S_Attribute Structure"))
  (locals (LocalAttributeFound :type "/Game/Dynamic/Blueprints/RPG_Systems/Attributes/S_Attribute Structure"))
  (`self.DetermineAttribute` TagSearchedFor
    (:`Health`
      (bind _output_get (set `local.LocalAttributeFound` (`self.Health`)))
      (return _output_get))))