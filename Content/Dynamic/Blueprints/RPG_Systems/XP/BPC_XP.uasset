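; BPC_XP is an actor component that handles experience and leveling, both earning XP and granting it on death.
; When BPC_GameplayTags reports State.Dead on the owner, it awards XPToAward to the BPC_XP on the originating controller's pawn.
; AwardXP recursively levels up against LevelCurve until MaxLevel, with ShouldLevelUp incrementing CurrentLevel itself.
; LevelUp and XPChanged dispatchers broadcast progress, though XPChanged always sends level 0.
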(event `self.ReceiveBeginPlay`
  (`/Game/Dynamic/Blueprints/RPG_Systems/GameplayTags/BPC_GameplayTags.AddTagListener` (`Actor.GetComponentByClass` (`self.GetOwner`) "/Game/Dynamic/Blueprints/RPG_Systems/GameplayTags/BPC_GameplayTags.BPC_GameplayTags_C") (struct :`TagName` "State.Dead") (delegate `DeadStateUpdate`)))

(event `DeadStateUpdate`
  (params (GameplayTagContext :type "/Game/Dynamic/Blueprints/S_GameplayContext Structure"))
  (bind (_contexttag _activetags _origin) (break `/Game/Dynamic/Blueprints/S_GameplayContext` GameplayTagContext))
  (bind (_actor _controller) (break `/Game/Dynamic/Blueprints/S_Origin` _origin))
  (bind _returnvalue (`Actor.GetComponentByClass` (`Controller.K2_GetPawn` _controller) "BPC_XP_C"))
  (if (`BlueprintGameplayTagLibrary.HasTag` _activetags (struct :`TagName` "State.Dead"))
    (`/Engine/EditorBlueprintResources/StandardMacros.IsValid` _controller
      (:`Is Valid`
        (`/Engine/EditorBlueprintResources/StandardMacros.IsValid` _returnvalue
          (:`Is Valid`
            (`self.AwardXP` _returnvalue (`self.XP_to_Award`))))))))

(event `AwardXP`
  (params (AwardedXP :type "Float (double-precision)"))
  (bind _output_get (set `self.CurrentXP` (+ (`self.CurrentXP`) AwardedXP)))
  (`self.TryToLevelUp`)
  (`self.XPChanged` (make `/Game/Dynamic/Blueprints/RPG_Systems/XP/S_XPContext` _output_get)))

(event `Signature` :!signature `self.XPChanged`
  (params (XPContext :type "/Game/Dynamic/Blueprints/RPG_Systems/XP/S_XPContext Structure")))

(fn `ShouldLevelUp?`
  (returns (LeveledUp :type Boolean))
  (if (== (`self.CurrentLevel`) (`self.MaxLevel`))
    (return false)
    (elif (>= (`self.CurrentXP`) (`CurveFloat.GetFloatValue` (`self.LevelCurve`) (`KismetMathLibrary.Conv_IntToDouble` (+ (`self.CurrentLevel`) 1))))
      (`/Engine/EditorBlueprintResources/StandardMacros.IncrementInt` (`self.CurrentLevel`)
        (:`  `
          (return true)))
      (else
        (return false)))))

(fn `TryToLevelUp`
  (bind _leveledup (`self.ShouldLevelUp?`))
  (if _leveledup
    (`self.LevelUp` (make `/Game/Dynamic/Blueprints/RPG_Systems/XP/S_XPContext` (`self.CurrentXP`) (`self.CurrentLevel`)))
    (`KismetSystemLibrary.PrintString` "Level Up!")
    (`GameplayStatics.PlaySound2D` "/Engine/EditorSounds/Notifications/CompileStart_Cue.CompileStart_Cue" 1.0 1.0 0.0 null null)
    (`self.TryToLevelUp`)
    (return)
    (else
      (return))))